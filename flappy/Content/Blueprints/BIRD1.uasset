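; BIRD1 is a Flappy Bird-style side-scrolling bird actor, represented by a sphere that flaps on Space and is destroyed on a hit.
; Tick sweeps the sphere along world X at the Hitrost speed and moves the camera to its X with a fixed Y offset, without following its height.
; Space sets an upward physics velocity for each flap, and any component hit on the sphere destroys the whole actor.
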(event OnComponentHit(Sphere)
  (params (HitComponent :type Primitive%20Component%20Object%20Reference) (OtherActor :type Actor%20Object%20Reference) (OtherComp :type Primitive%20Component%20Object%20Reference) (NormalImpulse :type Vector :default "0, 0, 0") (Hit :type Hit%20Result%20Structure%20%28by%20ref%29))
  (Actor|DestroyActor))

(event EventBeginPlay)

(event Collision|EventActorBeginOverlap
  (params (OtherActor :type Actor%20Object%20Reference)))

(event EventTick
  (params (DeltaSeconds :type Float%20%28single-precision%29))
  (bind _sphere (Variables|Default|GetSphere))
  (bind _returnvalue (Transformation|GetWorldLocation _sphere))
  (Utilities|IsValid (Variables|Default|GetSphere)
    (:Is%20Valid
      (Transformation|AddWorldOffset (Variables|Default|GetSphere) (Math|Vector|MakeVector (* DeltaSeconds (Variables|Default|Gethitrost)) 0.0 0.0) true false)
      (Utilities|IsValid (Variables|Default|GetSphere)
        (:Is%20Valid
          (Utilities|IsValid (Variables|Default|GetCamera)
            (:Is%20Valid
              (Transformation|SetWorldLocation (Variables|Default|GetCamera) (Math|Vector|MakeVector (.x _returnvalue) (+ (.y _returnvalue) 1e+03) 0.0) false false))))))))

(event Input|KeyboardEvents|SpaceBar
  (params (Key :type Key%20Structure :default "None"))
  (:Pressed
    (Physics|SetPhysicsLinearVelocity (Variables|Default|GetSphere) (Math|Vector|MakeVector 0.0 0.0 5e+02) false "None")))

(fn ConstructionScript)