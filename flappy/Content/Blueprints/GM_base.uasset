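; Base game mode, by its name, for a Flappy Bird-style game that spawns and possesses the bird and generates the pipe course.
; BeginPlay places BIRD1 at the first PlayerStart, pre-spawns several pipes and starts a looping spawn timer.
; Spawn spaces pipes evenly along X with a bounded random-walk height, recursively rerolling out-of-range values.
; Restart destroys all pipes, resets the counter and last height, then re-enters the BeginPlay setup.
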(event Custom|spawn
  (Variables|Default|SetnewZ (+ (Math|Random|RandomIntegerinRange -150 150) (Variables|Default|Getprejšnja%20Z)))
  (if (and (< (Variables|Default|GetnewZ) 250) (> (Variables|Default|GetnewZ) -250))
    (bind _returnvalue (Game|SpawnActorfromClass "/Game/Blueprints/PIPE.PIPE_C" (Math|Transform|MakeTransform (Math|Vector|MakeVector (Math|Conversions|ToFloat(Integer) (* (Variables|Default|Getstevec) 800)) 0.0 (Math|Conversions|ToFloat(Integer) (Variables|Default|GetnewZ))) "0, 0, 0" "1,1,1") "Undefined" 0 0))
    (Math|Integer|IncrementInt (Variables|Default|Getstevec)
      (:%20%20
        (Variables|Default|Setprejšnja%20Z (Math|Float|Truncate (.z (Transformation|GetActorLocation _returnvalue))))))
    (else
      (CallFunction|Spawn))))

(event Custom|restart
  (bind _outactors (Actor|GetAllActorsOfClass "/Game/Blueprints/PIPE.PIPE_C"))
  (Actor|DestroyActor _outactors)
  (Utilities|FlowControl|Sequence
    (:then_0
      (Variables|Default|Setstevec 0)
      (Variables|Default|Setprejšnja%20Z 0))
    (:then_1
      (bind _outactors_2 (Actor|GetAllActorsOfClass "/Script/Engine.PlayerStart"))
      (bind _returnvalue (Game|SpawnActorfromClass "/Game/Blueprints/BIRD1.BIRD1_C" (Math|Transform|MakeTransform (Transformation|GetActorLocation (Utilities|Array|Get(acopy) _outactors_2)) "0, 0, 0" "1,1,1") "Undefined" 0 0))
      (Pawn|Possess (Game|GetPlayerController 0) _returnvalue)
      (for _index (range 0 4)
        (CallFunction|Spawn))
      (Utilities|Time|SetTimerbyEvent (delegate Custom|spawn) 1.0 true))))

(event EventBeginPlay
  (bind _outactors (Actor|GetAllActorsOfClass "/Script/Engine.PlayerStart"))
  (bind _returnvalue (Game|SpawnActorfromClass "/Game/Blueprints/BIRD1.BIRD1_C" (Math|Transform|MakeTransform (Transformation|GetActorLocation (Utilities|Array|Get(acopy) _outactors)) "0, 0, 0" "1,1,1") "Undefined" 0 0))
  (Pawn|Possess (Game|GetPlayerController 0) _returnvalue)
  (for _index (range 0 4)
    (CallFunction|Spawn))
  (Utilities|Time|SetTimerbyEvent (delegate Custom|spawn) 1.0 true))

(event EventTick
  (params (DeltaSeconds :type Float%20%28single-precision%29)))

(fn ConstructionScript)